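; Game mode that sets how many gun-holding enemies remain in the map at the start of play, based on difficulty.
; On BeginPlay it reads Difficulty from the PersistentSettings game instance and sets EnemiesInMap to twice its truncated value.
; It then shuffles all placed Enemy_Holding_Gun actors and destroys the surplus, leaving a random subset and storing the remaining count in TotalEnemies.
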(event EventBeginPlay
  (Utilities|FlowControl|Sequence
    (:then_0
      (bind _aspersistent_settings (Utilities|Casting|CastToPersistentSettings (Game|GetGameInstance)))
      (Variables|Default|SetEnemies%20In%20Map (* (Math|Float|Truncate (Variables|/Game/UI/PersistentSettings.PersistentSettings_C|GetDifficullty _aspersistent_settings)) 2)))
    (:then_1
      (bind _outactors (Actor|GetAllActorsOfClass "/Game/AnimStarterPack/Enemy_Holding_Gun.Enemy_Holding_Gun_C"))
      (Utilities|Array|Shuffle _outactors)
      (Variables|Default|SetTotalEnemies (Utilities|Array|Length _outactors))
      (for _index (range 0 (- (Utilities|Array|Length _outactors) (+ (Variables|Default|GetEnemies%20In%20Map) 1)))
        (Actor|DestroyActor (Utilities|Array|Get(acopy) _outactors _index))
        (Variables|Default|SetTotalEnemies (- (Variables|Default|GetTotalEnemies) 1))))))

(fn ConstructionScript)