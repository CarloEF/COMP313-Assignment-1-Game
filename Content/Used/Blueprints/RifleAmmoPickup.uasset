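; Rifle ammo pickup actor that raises the MaxAmmo of the overlapping MyCharacter's equipped weapon by a fixed amount.
; On overlap it plays a small explosion effect and sound, then hides and disables collision and tick until a timed delay respawns it.
; On BeginPlay it disables itself the same way when the GameInstance's PersistentSettings has GenerateInteractables off.
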(event EventBeginPlay
  (bind _aspersistent_settings (Utilities|Casting|CastToPersistentSettings (Game|GetGameInstance)))
  (if (not (Variables|/Game/UI/PersistentSettings.PersistentSettings_C|GetGenerateInteractables _aspersistent_settings))
    (Rendering|SetActorHiddenInGame true)
    (Collision|SetActorEnableCollision false)
    (Actor|Tick|SetActorTickEnabled false)))

(event Collision|EventActorBeginOverlap
  (params (OtherActor :type Actor%20Object%20Reference))
  (bind _asmy_character (Utilities|Casting|CastToMyCharacter OtherActor))
  (Variables|/Game/Used/Blueprints/Weapons/AK-47/Weapon_Base.Weapon_Base_C|SetMaxAmmo (Variables|/Game/Used/Blueprints/MyCharacter.MyCharacter_C|GetEquippedWeapon _asmy_character) (+ (Variables|/Game/Used/Blueprints/Weapons/AK-47/Weapon_Base.Weapon_Base_C|GetMaxAmmo (Variables|/Game/Used/Blueprints/MyCharacter.MyCharacter_C|GetEquippedWeapon _asmy_character)) 60))
  (Effects|SpawnEmitteratLocation "/Game/InfinityBladeEffects/Effects/FX_Monsters/FX_Monster_Gruntling/Bomber/P_BomberExplode.P_BomberExplode" (Transformation|GetActorLocation) "0, 0, 0" "0.300000,0.300000,0.300000")
  (Audio|SpawnSoundatLocation "/Game/StarterContent/Audio/Explosion01.Explosion01" (Transformation|GetActorLocation) "0, 0, 0" 1.0 1.0 0.0 0 0)
  (Rendering|SetActorHiddenInGame true)
  (Collision|SetActorEnableCollision false)
  (Actor|Tick|SetActorTickEnabled false)
  (Utilities|FlowControl|Delay 15.0)
  (Rendering|SetActorHiddenInGame false)
  (Collision|SetActorEnableCollision true)
  (Actor|Tick|SetActorTickEnabled true))

(fn ConstructionScript)