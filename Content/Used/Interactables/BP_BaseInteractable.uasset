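; BP_BaseInteractable is a base interactable Blueprint with a trigger area and a highlightable mesh.
; Beginning overlap with InteractableArea registers it with MyCharacter, while end overlap only casts, leaving the unregister call unconnected.
; SetHighlight toggles the mesh's custom depth rendering.
; The Interact input prints a debug string without checking overlap.
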(event OnComponentBeginOverlap(InteractableArea)
  (params (OverlappedComponent :type Primitive%20Component%20Object%20Reference) (OtherActor :type Actor%20Object%20Reference) (OtherComp :type Primitive%20Component%20Object%20Reference) (OtherBodyIndex :type Integer) (bFromSweep :type Boolean) (SweepResult :type Hit%20Result%20Structure%20%28by%20ref%29))
  (bind _asmy_character (Utilities|Casting|CastToMyCharacter OtherActor))
  (Class|BPIInteract|RegisterInteractable(Message) _asmy_character self))

(event OnComponentEndOverlap(InteractableArea)
  (params (OverlappedComponent :type Primitive%20Component%20Object%20Reference) (OtherActor :type Actor%20Object%20Reference) (OtherComp :type Primitive%20Component%20Object%20Reference) (OtherBodyIndex :type Integer))
  (bind _asmy_character (Utilities|Casting|CastToMyCharacter OtherActor)))

(event Input|ActionEvents|InputActionInteract
  (params (Key :type Key%20Structure :default "None"))
  (:Pressed
    (Development|PrintString "I've been interacted with")))

(fn ConstructionScript)

(fn SetHighlight
  (params (Highlight? :type Boolean))
  (Rendering|SetRenderCustomDepth (Variables|Default|GetInteractableMesh) Highlight?))